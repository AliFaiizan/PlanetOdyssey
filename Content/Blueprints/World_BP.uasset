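; World_BP is a touch-controlled globe that serves as a level selection map.
; On BeginPlay it caches UmgManager_BP and plays a timeline that eases the spring arm to a set zoom distance.
; The globe spins constantly on Tick, while touch drags rotate it by the frame-to-frame screen position delta.
; Touching the ForrestLvl1 marker sets SelectedLevel and has the UMG manager create the location menu.
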(event OnInputTouchBegin(forrestlvl1)
  (params (FingerIndex :type ETouchIndex%20Enum :default "Touch1") (TouchedComponent :type Primitive%20Component%20Object%20Reference))
  (Development|PrintString "Hello")
  (Variables|Default|Setselected%20level 1)
  (Default|CreateLocationMenu (Variables|Default|GetUmg_manager)))

(event EventBeginPlay
  (bind _outactors (Actor|GetAllActorsOfClass "/Game/Blueprints/UmgManager_BP.UmgManager_BP_C"))
  (Variables|Default|SetUmg_manager (Utilities|Array|Get(acopy) _outactors))
  (bind _move_alpha (Timeline|camera%20movement PlayFromStart)
    (:Update
      (Variables|/Script/Engine.SpringArmComponent|SetTargetArmLength (Variables|Default|GetSpringArm) (Math|Float|Lerp (Variables|/Script/Engine.SpringArmComponent|GetTargetArmLength (Variables|Default|GetSpringArm)) 1.7e+02 _move_alpha)))))

(event Collision|EventActorBeginOverlap
  (params (OtherActor :type Actor%20Object%20Reference)))

(event EventTick
  (params (DeltaSeconds :type Float%20%28single-precision%29))
  ;[1 1 1] constant rotation
  (Transformation|AddWorldRotation (Variables|Default|Getworld%20mesh) (Math|Rotator|MakeRotator 0.0 0.0 (Variables|Default|Getglobe%20speed)) false false))

(event Input|TouchEvents|InputTouch
  (params (Location :type Vector) (FingerIndex :type ETouchIndex%20Enum))
  ;[1 1 1] touch controll
  (:Pressed
    (Variables|Default|SetStartPosition (CallFunction|GetClickPosition)))
  (:Moved
    (Variables|Default|SetEndPosition (CallFunction|GetClickPosition))
    (Transformation|AddWorldRotation (Variables|Default|Getworld%20mesh) (Math|Rotator|MakeRotator 0.0 (* (* (Variables|Default|GetrotationSpeed) (Utilities|Time|GetWorldDeltaSeconds) (.y (- (Variables|Default|GetStartPosition) (Variables|Default|GetEndPosition)))) -1.0) (* (Variables|Default|GetrotationSpeed) (Utilities|Time|GetWorldDeltaSeconds) (.x (- (Variables|Default|GetStartPosition) (Variables|Default|GetEndPosition))))) false false)
    (Variables|Default|SetStartPosition (CallFunction|GetClickPosition))))

(fn ConstructionScript)

(fn GetClickPosition
  (bind _returnvalue (Game|GetPlayerController 0))
  (bind (_locationx _locationy) (Class|PlayerController|GetInputTouchState _returnvalue "Touch1"))
  (return (Math|Vector2D|MakeVector2D _locationx _locationy)))