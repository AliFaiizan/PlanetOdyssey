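; UMG manager actor that shows the main UI on BeginPlay and spawns location menus for levels or information entries.
; BeginPlay caches the World_BP actor, then creates the Main widget and plays its intro animation.
; CreateLocationMenu switches on an index to build a level or info widget, fill it from the passed data and animate it in.
; Level menus also get generated objective rows and pass the target level to the play button.
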(event Custom|Create%20Location%20Menu
  (params (Selected%20index :type Integer) (Level%20Data :type Forrest%20Data%20Structure) (Information%20Data :type Information%20Data%20Structure))
  (switch int Selected%20index
    (:0
      (CallFunction|CreateLevelWidget)
      (CallFunction|InsertLevelData Level%20Data))
    (:1
      (CallFunction|CreateInformationWidget)
      (CallFunction|InsertInformationData Information%20Data))))

(event EventBeginPlay
  (bind _outactors (Actor|GetAllActorsOfClass "/Game/Blueprints/World_BP.World_BP_C"))
  (Variables|Default|Setworld%20ref (Utilities|Array|Get(acopy) _outactors))
  (bind _returnvalue (UserInterface|CreateWidget "/Game/Widgets/Main.Main_C" (Game|GetPlayerController 0)))
  (UserInterface|Viewport|AddtoViewport _returnvalue 0)
  (UserInterface|Animation|PlayAnimation _returnvalue (Variables|/Game/Widgets/Main.Main_C|Getinit _returnvalue) 0.0 1 "Forward" 0.5))

(event Collision|EventActorBeginOverlap
  (params (OtherActor :type Actor%20Object%20Reference)))

(fn ConstructionScript)

(fn CreateLevelWidget
  (bind _returnvalue (UserInterface|CreateWidget "/Game/Widgets/W_Level_Info.W_Level_Info_C"))
  (Variables|Default|SetLevel%20Widget _returnvalue))

(fn CreateInformationWidget
  (bind _returnvalue (UserInterface|CreateWidget "/Game/Widgets/W_Information.W_Information_C"))
  (Variables|Default|SetInfoWidget _returnvalue))

(fn InsertLevelData
  (params (Level%20Data :type Forrest%20Data%20Structure))
  (bind (_leveltitle _leveldetail _levelimage _levelobjectives _leveltoload) (Utilities|Struct|BreakForrestData Level%20Data))
  (bind _level_widget (Variables|Default|GetLevel%20Widget))
  (bind _level_widget_2 (Variables|Default|GetLevel%20Widget))
  (Utilities|FlowControl|Sequence
    (:then_0
      (Rendering|Components|TextRender|SetText (Variables|/Game/Widgets/W_Level_Info.W_Level_Info_C|GetLevelName _level_widget_2) (Utilities|Text|ToText(String) _leveltitle)))
    (:then_1
      (Rendering|Components|TextRender|SetText (Variables|/Game/Widgets/W_Level_Info.W_Level_Info_C|GetLevelDetail _level_widget_2) _leveldetail))
    (:then_2
      (Class|Image|SetBrush (Variables|/Game/Widgets/W_Level_Info.W_Level_Info_C|GetLevelImage _level_widget_2) (Utilities|Struct|MakeSlateBrush "(X=32.000000,Y=32.000000)" "(Left=0.000000,Top=0.000000,Right=0.000000,Bottom=0.000000)" "(SpecifiedColor=(R=1.000000,G=1.000000,B=1.000000,A=1.000000),ColorUseRule=UseColor_Specified)" _levelimage "Image" "NoTile" "NoMirror")))
    (:then_4
      (for _array_element _levelobjectives
        (bind _returnvalue (UserInterface|CreateWidget "/Game/Widgets/W_Text.W_Text_C"))
        (Widget|Panel|AddChild (Variables|/Game/Widgets/W_Level_Info.W_Level_Info_C|GetObjs (Variables|Default|GetLevel%20Widget)) _returnvalue)
        (Rendering|Components|TextRender|SetText (Variables|/Game/Widgets/W_Text.W_Text_C|GetObjectiveText _returnvalue) (Utilities|Text|ToText(String) _array_element))))
    (:then_5
      (Variables|/Game/Widgets/W_Button.W_Button_C|SetLevel%20to%20load (Variables|/Game/Widgets/W_Level_Info.W_Level_Info_C|GetPlayButton (Variables|Default|GetLevel%20Widget)) _leveltoload))
    (:then_6
      (UserInterface|Viewport|AddtoViewport _level_widget 0)
      (UserInterface|Animation|PlayAnimation _level_widget (Variables|/Game/Widgets/W_Level_Info.W_Level_Info_C|GetStartAnimation _level_widget) 0.0 1 "Forward" 1.0))))

(fn InsertInformationData
  (params (info :type Information%20Data%20Structure))
  (bind (_heading _detail) (Utilities|Struct|BreakInformationData info))
  (bind _infowidget (Variables|Default|GetInfoWidget))
  (Utilities|FlowControl|Sequence
    (:then_0
      (Rendering|Components|TextRender|SetText (Variables|/Game/Widgets/W_Information.W_Information_C|GetInfoHeading _infowidget) (Utilities|Text|ToText(String) _heading)))
    (:then_1
      (Rendering|Components|TextRender|SetText (Variables|/Game/Widgets/W_Information.W_Information_C|GetInfoDetail _infowidget) _detail))
    (:then_2
      (UserInterface|Viewport|AddtoViewport _infowidget 0)
      (UserInterface|Animation|PlayAnimation _infowidget (Variables|/Game/Widgets/W_Information.W_Information_C|GetTextAnimation _infowidget) 0.0 1 "Forward" 1.0))))