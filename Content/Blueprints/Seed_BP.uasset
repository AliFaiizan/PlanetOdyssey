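; Physics seed actor that, once launched, comes to rest and grows into a tree or disappears, and can be picked up by a SeedCollector.
; A timeline scales the mesh on spawn, while Tick halts slow movement, then traces down once to read the physical surface.
; After a delay, grass or soil spawns Tree_BP.
; Landing and collection both destroy the seed, decrement PlanetGameMode's seed count and check the game condition.
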(event OnComponentBeginOverlap(SeedMesh)
  (params (OverlappedComponent :type Primitive%20Component%20Object%20Reference) (OtherActor :type Actor%20Object%20Reference) (OtherComp :type Primitive%20Component%20Object%20Reference) (OtherBodyIndex :type Integer) (bFromSweep :type Boolean) (SweepResult :type Hit%20Result%20Structure%20%28by%20ref%29))
  (Variables|Default|SetbIsLaunched false)
  (bind _asseed_collector_bp (Utilities|Casting|CastToSeedCollector_BP OtherActor))
  (Default|SeedUpdate _asseed_collector_bp 1)
  (Actor|DestroyActor)
  (bind _asplanet_game_mode (Utilities|Casting|CastToPlanetGameMode (Game|GetGameMode)))
  (bind _result (Math|Integer|DecrementInt (Variables|/Game/PlanetGameMode.PlanetGameMode_C|GetTotal%20Available%20Seed _asplanet_game_mode))
    (:%20%20
      (Variables|/Game/PlanetGameMode.PlanetGameMode_C|SetTotal%20Available%20Seed _asplanet_game_mode _result)
      (Default|UpdateSeed _asplanet_game_mode)
      (Default|CheckGameCondition _asplanet_game_mode))))

(event EventBeginPlay
  (bind _seedmesh (Variables|Default|GetSeedMesh))
  (bind _time (Timeline|Spawn%20Animation PlayFromStart)
    (:Update
      (Transformation|SetWorldScale3D _seedmesh (Math|Vector|Lerp(Vector) (Transformation|GetWorldScale _seedmesh) "0.200000,0.200000,0.200000" _time)))))

(event Collision|EventActorBeginOverlap
  (params (OtherActor :type Actor%20Object%20Reference)))

(event EventTick
  (params (DeltaSeconds :type Float%20%28single-precision%29))
  (bind _seedmesh (Variables|Default|GetSeedMesh))
  (bind _seedmesh_2 (Variables|Default|GetSeedMesh))
  (bind _seedmesh_3 (Variables|Default|GetSeedMesh))
  (bind _returnvalue (Transformation|GetWorldLocation _seedmesh))
  (bind _returnvalue_2 (Transformation|GetWorldTransform _seedmesh_3))
  (if (<= (Math|Vector|VectorLength (Transformation|GetComponentVelocity (Variables|Default|GetSeedMesh))) 2e+01)
    (Physics|SetPhysicsLinearVelocity _seedmesh_2 "0, 0, 0" false "None")
    (if (and (Variables|Default|GetbIsLaunched) (<= (Math|Vector|VectorLength (Transformation|GetComponentVelocity _seedmesh_2)) 2.0))
      (bind _outhit (Collision|LineTraceByChannel _returnvalue (+ _returnvalue "0,0.000000,-50.000000") "TraceTypeQuery1" false 0 "Persistent"))
      (Utilities|FlowControl|DoOnce false
        (:Completed
          (Utilities|FlowControl|Delay 1.0)
          (switch Utilities|FlowControl|Switch|SwitchonEPhysicalSurface (Variables|/Script/Engine.PhysicalMaterial|GetSurfaceType (.PhysMat (Collision|BreakHitResult _outhit)))
            (:SurfaceType_Default
              (Actor|DestroyActor))
            (:SurfaceType1
              (Game|SpawnActorfromClass "/Game/Blueprints/Tree_Bp.Tree_BP_C" (Math|Transform|MakeTransform (.location _returnvalue_2) "0, 0, 0" "1,1,1") "AlwaysSpawn" 0 0)
              (Actor|DestroyActor :!label _label))
            (:SurfaceType2
              (Game|SpawnActorfromClass "/Game/Blueprints/Tree_Bp.Tree_BP_C" (Math|Transform|MakeTransform (.location _returnvalue_2) "0, 0, 0" "1,1,1") "AlwaysSpawn" 0 0)
              (goto _label))
            (:SurfaceType3
              (Actor|DestroyActor :!label _label_2))
            (:SurfaceType4
              (goto _label_2)))
          (bind _asplanet_game_mode (Utilities|Casting|CastToPlanetGameMode (Game|GetGameMode)))
          (bind _result (Math|Integer|DecrementInt (Variables|/Game/PlanetGameMode.PlanetGameMode_C|GetTotal%20Available%20Seed _asplanet_game_mode))
            (:%20%20
              (Variables|/Game/PlanetGameMode.PlanetGameMode_C|SetTotal%20Available%20Seed _asplanet_game_mode _result)
              (Default|UpdateSeed _asplanet_game_mode)
              (Default|CheckGameCondition _asplanet_game_mode))))))))

(fn ConstructionScript)