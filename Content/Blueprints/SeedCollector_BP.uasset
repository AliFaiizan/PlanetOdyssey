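; Seed collector actor that tallies delivered seeds and triggers the win condition once the total is reached.
; SeedUpdate adds the passed amount, then either plays a sound and refreshes the collected/total text, or shows the win menu, calls its Rewards and sets GameWon on PlanetGameMode.
; Each tick, the SeedAmount text rotates to face the player's pawn.
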(event Custom|Seed%20Update
  (params (NewParam :type Integer))
  (bind _total_seed (Variables|Default|Gettotal%20seed))
  (bind _output_get (Variables|Default|SetCollected%20seed (+ (Variables|Default|GetCollected%20seed) NewParam)))
  (if (>= _output_get _total_seed)
    (Audio|PlaySound2D "/Game/Audio/positive_action.positive_action" 1.0 1.0 0.0 0 0)
    (bind _returnvalue (UserInterface|CreateWidget "/Game/Widgets/W_WinMenu.W_WinMenu_C"))
    (UserInterface|Viewport|AddtoViewport _returnvalue 0)
    (Default|Rewards _returnvalue)
    (Variables|/Game/PlanetGameMode.PlanetGameMode_C|SetGame%20Won (Variables|Default|GetplanetGameMode) true)
    (else
      (Audio|PlaySound2D "/Game/Audio/itemize.itemize" 1.0 1.0 0.0 0 0)
      (Rendering|Components|TextRender|SetText (Variables|Default|GetSeed%20Amount) (Utilities|Text|FormatText "{Collected Seed}/{Total Seed}" _output_get _total_seed)))))

(event EventBeginPlay
  (bind _asplanet_game_mode (Utilities|Casting|CastToPlanetGameMode (Game|GetGameMode)))
  (Variables|Default|SetplanetGameMode _asplanet_game_mode))

(event Collision|EventActorBeginOverlap
  (params (OtherActor :type Actor%20Object%20Reference)))

(event EventTick
  (params (DeltaSeconds :type Float%20%28single-precision%29))
  (bind _seed_amount (Variables|Default|GetSeed%20Amount))
  (Transformation|SetWorldRotation _seed_amount (Math|Rotator|FindLookatRotation (Transformation|GetWorldLocation _seed_amount) (Transformation|GetActorLocation (Pawn|GetControlledPawn (Game|GetPlayerController 0)))) false false))

(fn ConstructionScript)