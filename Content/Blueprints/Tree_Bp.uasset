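; Tree actor that grows on spawn, then bears a random number of seeds that can be thrown toward a target location.
; A timeline on BeginPlay scales the trunk and leaves to full size, then spawns Seed_BP actors at arrow components.
; ThrowSeed launches the next stored seed by yawing it toward the target, setting horizontal physics velocity and enabling simulation, clearing HasSeed once all are used.
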(event Custom|Spawn%20Seeds
  (bind _locations (CallFunction|LocationtoSpawnSeed))
  (for _index (range 0 (Variables|Default|GetNumber%20of%20Seed))
    (bind _returnvalue (Game|SpawnActorfromClass "/Game/Blueprints/Seed_BP.Seed_BP_C" (Utilities|Array|Get(acopy) _locations _index) "AlwaysSpawn" 0 0))
    (Utilities|Array|Add (Variables|Default|GetSpawned%20Seed) _returnvalue)
    (Variables|Default|SetbHasSeed true)))

(event Custom|Throw%20Seed
  (params (Direction :type Vector))
  (if (Variables|Default|GetbHasSeed)
    (Development|PrintString (Utilities|String|ToString(Vector) Direction))
    (Variables|/Game/Blueprints/Seed_BP.Seed_BP_C|SetbIsLaunched (Utilities|Array|Get(acopy) (Variables|Default|GetSpawned%20Seed) (Variables|Default|Gettest)) true)
    (Transformation|SetActorRotation (Utilities|Array|Get(acopy) (Variables|Default|GetSpawned%20Seed) (Variables|Default|Gettest)) (Math|Rotator|MakeRotator 0.0 0.0 (.yaw (Math|Rotator|MakeRotfromX (Math|Vector|GetUnitDirection(Vector) (Transformation|GetActorLocation) Direction)))))
    (Physics|SetPhysicsLinearVelocity (Variables|/Game/Blueprints/Seed_BP.Seed_BP_C|GetSphere (Utilities|Array|Get(acopy) (Variables|Default|GetSpawned%20Seed) (Variables|Default|Gettest))) (Math|Vector|MakeVector (.x (* (Transformation|GetActorForwardVector (Utilities|Array|Get(acopy) (Variables|Default|GetSpawned%20Seed) (Variables|Default|Gettest))) 1.2e+03)) (.y (* (Transformation|GetActorForwardVector (Utilities|Array|Get(acopy) (Variables|Default|GetSpawned%20Seed) (Variables|Default|Gettest))) 1.2e+03)) 0.0) false "None")
    (Physics|SetSimulatePhysics (Variables|/Game/Blueprints/Seed_BP.Seed_BP_C|GetSphere (Utilities|Array|Get(acopy) (Variables|Default|GetSpawned%20Seed) (Variables|Default|Gettest))) true)
    (bind _result (Math|Integer|IncrementInt (Variables|Default|Gettest))
      (:%20%20
        (Variables|Default|Settest _result)
        (bind _result_2 (Math|Integer|DecrementInt (Variables|Default|GetNumber%20of%20Seed))
          (:%20%20
            (bind _output_get (Variables|Default|SetNumber%20of%20Seed _result_2))
            (if (< _output_get 0)
              (Variables|Default|SetbHasSeed false))))))))

(event EventBeginPlay
  (bind _lower_part (Variables|Default|GetLower%20Part))
  (bind _leaves (Variables|Default|GetLeaves))
  (Variables|Default|SetNumber%20of%20Seed (Math|Random|RandomIntegerinRange 0 3))
  (bind _time (Timeline|Spawn%20Animtion PlayFromStart)
    (:Update
      (Transformation|SetWorldScale3D _lower_part (Math|Vector|Lerp(Vector) (Transformation|GetWorldScale _lower_part) "1.000000,1.000000,1.000000" _time))
      (Transformation|SetWorldScale3D _leaves (Math|Vector|Lerp(Vector) (Transformation|GetWorldScale _leaves) "1.000000,1.000000,1.000000" _time)))
    (:Finished
      (CallFunction|SpawnSeeds))))

(event Collision|EventActorBeginOverlap
  (params (OtherActor :type Actor%20Object%20Reference)))

(event EventTick
  (params (DeltaSeconds :type Float%20%28single-precision%29)))

(fn ConstructionScript)

(fn LocationtoSpawnSeed
  (return (Utilities|Array|MakeArray (Transformation|GetWorldTransform (Variables|Default|GetArrow)) (Transformation|GetWorldTransform (Variables|Default|GetArrow1)) (Transformation|GetWorldTransform (Variables|Default|GetArrow2)) (Transformation|GetWorldTransform (Variables|Default|GetArrow3)))))